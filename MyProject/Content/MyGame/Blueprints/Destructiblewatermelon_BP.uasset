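; A destructible watermelon actor that breaks apart when something overlaps its outer component.
; On the first overlap, guarded by a flag, it applies radius damage to the outer (外側) and inner (内側) destructible components at their own locations.
; It then increments the destruction count in MygameInstance, plays a bomb sound and destroys itself after a short delay.
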(event OnComponentBeginOverlap(外側)
  (params (OverlappedComponent :type Primitive%20Component%20Object%20Reference) (OtherActor :type Actor%20Object%20Reference) (OtherComp :type Primitive%20Component%20Object%20Reference) (OtherBodyIndex :type Integer) (bFromSweep :type Boolean) (SweepResult :type Hit%20Result%20Structure%20%28by%20ref%29))
  (bind _外側 (Variables|Default|Get外側))
  (bind _内側 (Variables|Default|Get内側))
  (if (not (Variables|Default|Getisdestroy))
    (Class|DestructibleComponent|ApplyRadiusDamage _外側 1e+02 (Transformation|GetWorldLocation _外側) 1e+02 1e+01 false)
    (Class|DestructibleComponent|ApplyRadiusDamage _内側 1e+02 (Transformation|GetWorldLocation _内側) 1e+02 1e+01 false)
    (Variables|Default|Setisdestroy true)
    (bind _asmygame_instance (Utilities|Casting|CastToMygameInstance (Game|GetGameInstance)))
    (Variables|/Game/MyGame/Blueprints/MygameInstance.MygameInstance_C|SetdestructNum _asmygame_instance (+ (Variables|/Game/MyGame/Blueprints/MygameInstance.MygameInstance_C|GetdestructNum _asmygame_instance) 1))
    (Audio|PlaySound2D "/Game/MyGame/sound/bomb.bomb" 1.0 1.0 0.0 0 0)
    (Utilities|FlowControl|Delay 1.0)
    (Actor|DestroyActor)))

(event EventBeginPlay)

(event Collision|EventActorBeginOverlap
  (params (OtherActor :type Actor%20Object%20Reference)))

(event EventTick
  (params (DeltaSeconds :type Float%20%28single-precision%29)))

(fn ConstructionScript)