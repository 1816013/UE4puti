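; Intact watermelon actor that breaks when its static mesh overlaps the Stick actor.
; On that hit it spawns Destructiblewatermelon_BP at the mesh's location and scale, decrements SpawnNum on the WatermelonSpawner, then destroys itself.
; Tick also destroys it once its world Y drops below a fixed limit, without touching the spawner count.
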(event OnComponentBeginOverlap(StaticMesh)
  (params (OverlappedComponent :type Primitive%20Component%20Object%20Reference) (OtherActor :type Actor%20Object%20Reference) (OtherComp :type Primitive%20Component%20Object%20Reference) (OtherBodyIndex :type Integer) (bFromSweep :type Boolean) (SweepResult :type Hit%20Result%20Structure%20%28by%20ref%29))
  (bind _staticmesh (Variables|Default|GetStaticMesh))
  (bind _returnvalue (Actor|GetActorOfClass "/Game/MyGame/Blueprints/stick.stick_C"))
  (if (== OtherActor _returnvalue)
    (Game|SpawnActorfromClass "/Game/MyGame/Blueprints/Destructiblewatermelon_BP.Destructiblewatermelon_BP_C" (Math|Transform|MakeTransform (Transformation|GetWorldLocation _staticmesh) "0, 0, 0" (Transformation|GetWorldScale _staticmesh)) "Undefined" 0 0)
    (bind _returnvalue_2 (Actor|GetActorOfClass "/Game/MyGame/Blueprints/watermelonSpawner.watermelonSpawner_C"))
    (Variables|/Game/MyGame/Blueprints/watermelonSpawner.watermelonSpawner_C|SetSpawnNum _returnvalue_2 (- (Variables|/Game/MyGame/Blueprints/watermelonSpawner.watermelonSpawner_C|GetSpawnNum _returnvalue_2) 1))
    (Actor|DestroyActor)))

(event EventBeginPlay)

(event Collision|EventActorBeginOverlap
  (params (OtherActor :type Actor%20Object%20Reference)))

(event EventTick
  (params (DeltaSeconds :type Float%20%28single-precision%29))
  (if (< (.y (.location (Transformation|GetActorTransform))) -3.5e+02)
    (Actor|DestroyActor)))

(fn ConstructionScript)