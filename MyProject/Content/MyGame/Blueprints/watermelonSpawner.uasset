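; Spawner Blueprint that scatters up to eight enlarged WatermelonStatic actors around the world origin.
; Tick checks SpawnNum and runs a Delay scaled by DeltaSeconds, so the spawn interval depends on frame rate.
; After each delay it increments the counter and spawns a melon at a random X/Y within 1000 units per axis, with Z held at zero.
; The counter never decreases here, so spawning stops once the cap is reached.
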(event EventTick
  (params (DeltaSeconds :type Float%20%28single-precision%29))
  (bind _returnvalue (Math|Random|RandomFloatinRange 0.0 1e+03))
  (bind _returnvalue_2 (Math|Random|RandomUnitVector))
  (bind _returnvalue_3 (* _returnvalue_2 _returnvalue))
  (if (< (Variables|Default|GetspawnNum) 8)
    (Utilities|FlowControl|Delay (* DeltaSeconds 1.8e+02))
    (Variables|Default|SetspawnNum (+ (Variables|Default|GetspawnNum) 1))
    (Game|SpawnActorfromClass "/Game/MyGame/Blueprints/watermelonStatic.watermelonStatic_C" (Math|Transform|MakeTransform (Math|Vector|MakeVector (.x _returnvalue_3) (.y _returnvalue_3) (* (.z _returnvalue_3) 0.0)) "0, 0, 0" "5.000000,5.000000,5.000000") "Undefined" 0 0)))

(event Collision|EventActorBeginOverlap
  (params (OtherActor :type Actor%20Object%20Reference)))

(event EventBeginPlay)

(fn ConstructionScript)