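; Sliceable watermelon actor that is cut in two when something overlaps it, counting the slice in the game instance.
; BeginPlay copies the static mesh into a procedural mesh.
; The first overlap slices it at the overlapping component's location along a plane derived from the player-to-mesh direction, capping the cut with a red material.
; The new half gets physics and an impulse, a sound plays, and the actor is destroyed shortly after.
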(event OnComponentBeginOverlap(ProceduralMesh)
  (params (OverlappedComponent :type Primitive%20Component%20Object%20Reference) (OtherActor :type Actor%20Object%20Reference) (OtherComp :type Primitive%20Component%20Object%20Reference) (OtherBodyIndex :type Integer) (bFromSweep :type Boolean) (SweepResult :type Hit%20Result%20Structure%20%28by%20ref%29))
  (bind _returnvalue (Game|GetPlayerCharacter 0))
  (bind _slicemesh (Variables|Default|GetSliceMesh))
  (bind _returnvalue_2 (Transformation|GetWorldLocation _slicemesh))
  (bind _mesh (Variables|/Script/Engine.Character|GetMesh _returnvalue))
  (bind _returnvalue_3 (Transformation|GetWorldLocation _mesh))
  (bind _returnvalue_4 (- _returnvalue_2 _returnvalue_3))
  (if (not (Variables|Default|GetisDestroy))
    (bind _outotherhalfprocmesh (Class|KismetProceduralMeshLibrary|SliceProceduralMesh (Variables|Default|GetProceduralMesh) (Transformation|GetWorldLocation OtherComp) (Math|Vector|MakeVector (* (.y _returnvalue_4) -1.0) (.x _returnvalue_4) 0.0) true "CreateNewSectionForCap" "/Game/MyGame/14_Watermelon_tguocjppa/redmaterial.redmaterial"))
    (Physics|SetSimulatePhysics _outotherhalfprocmesh true)
    (Physics|AddImpulse _outotherhalfprocmesh "1000.000000,1000.000000,1000.000000" "None" false)
    (Variables|Default|SetisDestroy true)
    (bind _asmygame_instance (Utilities|Casting|CastToMygameInstance (Game|GetGameInstance)))
    (Variables|/Game/MyGame/Blueprints/MygameInstance.MygameInstance_C|SetsliceNum _asmygame_instance (+ (Variables|/Game/MyGame/Blueprints/MygameInstance.MygameInstance_C|GetsliceNum _asmygame_instance) 1))
    (Audio|PlaySound2D "/Game/MyGame/sound/slice.slice" 1.0 1.0 0.0 0 0)
    (Utilities|FlowControl|Delay 1.0)
    (Actor|DestroyActor)))

(event EventBeginPlay
  (Class|KismetProceduralMeshLibrary|CopyProceduralMeshfromStaticMeshComponent (Variables|Default|GetSliceMesh) 0 (Variables|Default|GetProceduralMesh) false))

(event Collision|EventActorBeginOverlap
  (params (OtherActor :type Actor%20Object%20Reference)))

(event EventTick
  (params (DeltaSeconds :type Float%20%28single-precision%29)))

(fn ConstructionScript)